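; Construction actor that builds walls from spline meshes along a player-defined outline, entirely in the construction script.
; In Free Form mode, user points form an area spline, which is resampled at the default mesh's bounding-box X length into a wall spline.
; Each wall point gets a spline mesh using per-segment MeshData for mesh, curve type and forward axis.
; MeshData then resizes to the mesh count, and debug text numbers each point.
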(event `self.ReceiveBeginPlay`)

(fn `Generate Defalt`
  (bind _spline (`self.Spline`))
  (bind _meshdata (`self.MeshData`))
  (bind _splineparede (`self.SplineParede`))
  (`|ExecutionSequence`
    (:`then_0`
      ;[1 1 1] Seletor de Metodo
      (switch `/Game/MeuGame/BluePrints/BP/ConstructTypes` (`self.SelectConstructType`)
        (:`NewEnumerator0`
          ;[1 1 1] Gera Area Especificada Pelo Player
          (bind _returnvalue (`AddComponent|NODE_AddSplineComponent-1`))
          (bind _output_get (set `self.Spline` _returnvalue))
          (`SplineComponent.SetSplinePoints` _output_get (`self.Points`) "Local" true)
          (for _index (range (`SplineComponent.GetNumberOfSplinePoints` (`self.Spline`)))
            (`SplineComponent.SetSplinePointType` _spline _index (`self.SplinePointTypeAreaDefalt`) true))
          (`SplineComponent.SetClosedLoop` _spline (`self.In Closed Loop`) true)
          ;[1 1 1] Gera Area Automatizada das Paredes
          (`self.GenerateSpline`)
          ;[1 1 1] Spawn o Mesh PAREDE
          (`self.Generate Mesh`))))
    (:`then_1`
      ;[1 1 1] Criar DataMesh
      (`/Engine/EditorBlueprintResources/StandardMacros.CompareInt` (`KismetArrayLibrary.Array_Length` (`self.MeshData`)) (`KismetArrayLibrary.Array_Length` (`self.MalhasParedes`)) :!label _label
        (:`>`
          (`KismetArrayLibrary.Array_Remove` _meshdata (`KismetArrayLibrary.Array_LastIndex` _meshdata))
          (goto _label))
        (:`<`
          (`KismetArrayLibrary.Array_Add` (`self.MeshData`) (make `/Game/MeuGame/BluePrints/BP/ConstructData` (`self.MeshDefalt`) "Curve" (`self.Eixo De Avanço Defalt`)))
          (goto _label))))
    (:`then_2`
      ;[1 1 1] Cria Enumerador em Texto para as paredes (uso de Debug)
      (for _index_2 (range (`SplineComponent.GetNumberOfSplinePoints` _splineparede))
        (bind _returnvalue_2 (`AddComponent|NODE_AddTextRenderComponent-0` :`RelativeTransform` (`KismetMathLibrary.MakeTransform` (`SplineComponent.GetLocationAtSplinePoint` _splineparede _index_2 "Local"))))
        (`TextRenderComponent.K2_SetText` _returnvalue_2 (`KismetTextLibrary.Conv_IntToText` _index_2))))))

(fn `Generate Mesh`
  (bind _splineparede (`self.SplineParede`))
  (for _index (range (`SplineComponent.GetNumberOfSplinePoints` (`self.SplineParede`)))
    (bind _returnvalue (`AddComponent|NODE_AddSplineMeshComponent-0` :`bManualAttachment` true))
    (`KismetArrayLibrary.Array_Add` (`self.MalhasParedes`) _returnvalue)
    (bind (_location _tangent) (`SplineComponent.GetLocationAndTangentAtSplinePoint` _splineparede _index "World"))
    (bind (_location_2 _tangent_2) (`SplineComponent.GetLocationAndTangentAtSplinePoint` _splineparede (+ _index 1) "World"))
    (`SplineMeshComponent.SetStartAndEnd` _returnvalue _location _tangent _location_2 _tangent_2 true)
    (bind (_mesh _curvetype `_eixodeavanço`) (break `/Game/MeuGame/BluePrints/BP/ConstructData` (`|GetArrayItem` (`self.MeshData`) _index)))
    (`StaticMeshComponent.SetStaticMesh` _returnvalue _mesh)
    (`SplineMeshComponent.SetForwardAxis` _returnvalue `_eixodeavanço` true)))

(fn `GenerateSpline`
  (bind (_min _max) (break `Box` (`StaticMesh.GetBoundingBox` (`self.MeshDefalt`))))
  (bind _x (.x (- _max _min)))
  ;[1 0 0.01854] Corrigir sapoha Toda
  ;;[1 1 1] Entrada
  ;[1 1 1] Cria Os Pontos Para o Spline Parede
  (for _index (range (+ (`KismetMathLibrary.FTrunc` (/ (`SplineComponent.GetSplineLength` (`self.Spline`)) _x)) 1))
    (`KismetArrayLibrary.Array_Add` (`self.PointsRecalcule`) (`SplineComponent.GetLocationAtDistanceAlongSpline` (`self.Spline`) (* _index _x) "Local")))
  ;[1 1 1] Cria o Spline Parede 1 Andar
  (bind _returnvalue (`AddComponent|NODE_AddSplineComponent-4`))
  (bind _output_get (set `self.SplineParede` _returnvalue))
  (`SplineComponent.SetSplinePoints` _returnvalue (`self.PointsRecalcule`) "Local" true)
  (for _index_2 (range (`SplineComponent.GetNumberOfSplinePoints` _output_get))
    (`SplineComponent.SetSplinePointType` _output_get _index_2 (`.CurveType_5_95D113D741CBFBE6E29F8D97AEF64C17` (break `/Game/MeuGame/BluePrints/BP/ConstructData` (`|GetArrayItem` (`self.MeshData`) _index_2))) true))
  (`SplineComponent.SetClosedLoop` (`self.SplineParede`) (`self.In Closed Loop`) true))

(fn `UserConstructionScript`
  (`self.Generate Defalt`))